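; Apple tree actor whose mesh size reflects its Hits value.
; ScaleTree sets the static mesh's uniform world scale to Hits multiplied by DefaultScale, and runs on BeginPlay.
; ChangeHit stores a new Hits value and calls ScaleTree again, so the tree resizes whenever Hits is changed through it.
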(event EventBeginPlay
  (CallFunction|ScaleTree))

(event Collision|EventActorBeginOverlap
  (params (OtherActor :type Actor%20Object%20Reference)))

(event EventTick
  (params (DeltaSeconds :type Float%20%28single-precision%29)))

(fn ConstructionScript)

(fn ScaleTree
  (Transformation|SetWorldScale3D (Variables|Debug|GetStaticMeshComponent) (Math|Conversions|ToVector(Float) (* (Variables|Default|GetHits) (Variables|Default|GetDefaultScale)))))

(fn ChangeHit
  (params (NewHit :type Integer))
  (Variables|Default|SetHits NewHit)
  (CallFunction|ScaleTree))